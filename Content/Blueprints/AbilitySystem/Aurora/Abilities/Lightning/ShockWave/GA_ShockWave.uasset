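; Channeled lightning Gameplay Ability that beams from the caster's weapon to the target under the mouse, chaining to additional targets.
; After the montage event it locks movement, adds ShockLoop gameplay cues as beams, and starts a looping timer that commits cost and damages all targets.
; Input release (after a minimum hold), failed cost or primary-target death ends it, removing cues, applying final damage and committing cooldown.
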(event Custom|DamageAndCost
  (bind _returnvalue (Ability|CommitAbilityCost false))
  (if _returnvalue
    (CallFunction|ApplyDamage)
    (else
      ;[0.8702 0.2124 1] If Character out of mana
      (CallFunction|ClearTimeandEndAbility))))

(event Ability|EventActivateAbility
  (CallFunction|CombatInterfaceValidCheck)
  ;[0.1676 1 0.8802] Store Mouse Data Variables
  (bind _datahandle (|TargetDataUnderMouse)
    (:then
      (Class|AuroraBeamSpell|StoreMouseDataInfo (Ability|TargetData|GetHitResultfromTargetData _datahandle))
      (Class|AuroraBeamSpell|StoreOwnerPlayerVariables)
      (Utilities|FlowControl|Sequence
        (:then_0
          ;[1 0.6898 0.154] Facing Character Mesh towards to the target actor
          (Variables|/Script/Engine.PlayerController|SetbShowMouseCursor (Variables|Default|GetOwnerPC) false)
          (Class|CombatInterface|UpdateFacingTarget(Message) (Ability|GetAvatarActorfromActorInfo) (Variables|Default|GetMouseHitLocation)))
        (:then_1
          ;[0.4048 1 0.2977] Play ShockWave cast montage and wait for the Gameplay ability activate event
          (|PlayMontageandWaitProxy "None" (Variables|Default|GetMontage_Electocute) 1.0 "None" false 1.0 0.0 false
            (:then
              (Ability|Tasks|WaitGameplayEvent "(TagName=\"Event.Montage.Electrocute\")" 0 true
                (:EventReceived
                  (Utilities|FlowControl|Sequence
                    (:then_0
                      ;[1 1 1] Play Sound using GameplayCue
                      (GameplayCue|ExecuteGameplayCue :GameplayCueTag "(TagName=\"GameplayCue.ShockBurst\")"))
                    (:then_1
                      ;[0.3958 1 0.9275] Setup for Shock ability loop
                      (CallFunction|InShockLoop))
                    (:then_2
                      ;[0.02372 0.3523 1] Spawn Beam
                      (CallFunction|SpawnShockBeam))
                    (:then_3
                      (bind _returnvalue (Utilities|Time|SetTimerbyEvent (delegate Custom|DamageAndCost) (Variables|Default|GetDamageDeltaTime) true))
                      (Variables|Default|SetDamageAndCostTimer _returnvalue))))))))
        (:then_2
          ;[0.4531 0.7031 1] End up ability on input release
          (bind _timeheld (Ability|Tasks|WaitInputRelease false)
            (:OnRelease
              (Variables|Default|SetTime%20Held _timeheld)
              (if (< (Variables|Default|GetTime%20Held) (Variables|Default|GetMinSpellTime))
                (Utilities|FlowControl|Delay (- (Variables|Default|GetMinSpellTime) (Variables|Default|GetTime%20Held))))
              (CallFunction|ClearTimeandEndAbility))))))))

(event EventPrimaryTargetDied
  (params (DeadActor :type Actor%20Object%20Reference))
  (GameplayCue|RemoveGameplayCueOnActor(Looping) DeadActor "(TagName=\"GameplayCue.ShockLoop\")" (Variables|Default|GetFirstTargetCueParams))
  (CallFunction|ClearTimeandEndAbility))

(event EventAdditionalTargetDied
  (params (DeadActor :type Actor%20Object%20Reference))
  (CallFunction|RemoveLoopCurefromAddTarget DeadActor)
  (Utilities|Array|RemoveItem (Variables|Default|GetAdditionalTargets) DeadActor))

(fn CombatInterfaceValidCheck
  (if (not (Utilities|DoesObjectImplementInterface (Ability|GetAvatarActorfromActorInfo) "/Script/Aurora.CombatInterface"))
    (Ability|EndAbility)))

(fn PreparetoEndAbility
  (Utilities|FlowControl|Sequence
    (:then_0
      (Variables|/Script/Engine.PlayerController|SetbShowMouseCursor (Variables|Default|GetOwnerPC) true))
    (:then_1
      (Class|CombatInterface|SetinShockLoop(Message) (Ability|GetAvatarActorfromActorInfo) false))
    (:then_2
      (Pawn|Components|CharacterMovement|SetMovementMode (Variables|/Script/Engine.Character|GetCharacterMovement (Variables|Default|GetOwnerCharacter)) "MOVE_Walking" 0))
    (:then_3
      (if (Variables|Default|GetFirstTargetImplementsCombatInerface)
        (GameplayCue|RemoveGameplayCueOnActor(Looping) (Variables|Default|GetMouseHitActor) "(TagName=\"GameplayCue.ShockLoop\")" (Variables|Default|GetFirstTargetCueParams))
        (Class|AuroraAbilitySystemLibrary|ApplyDamageEffect (Class|AuroraDamageGameplayAbility|MakeDamageEffectParamsfromClassDefaults (Variables|Default|GetMouseHitActor) "0, 0, 0"))
        (else
          (GameplayCue|RemoveGameplayCueOnActor(Looping) (Ability|GetAvatarActorfromActorInfo) "(TagName=\"GameplayCue.ShockLoop\")" (Variables|Default|GetFirstTargetCueParams))))
      (for _array_element (Variables|Default|GetAdditionalTargets)
        (CallFunction|RemoveLoopCurefromAddTarget _array_element)
        (Class|AuroraAbilitySystemLibrary|ApplyDamageEffect (Class|AuroraDamageGameplayAbility|MakeDamageEffectParamsfromClassDefaults _array_element "0, 0, 0"))))))

(fn InShockLoop
  (Class|CombatInterface|SetinShockLoop(Message) (Ability|GetAvatarActorfromActorInfo) true)
  (Pawn|Components|CharacterMovement|DisableMovement (Variables|/Script/Engine.Character|GetCharacterMovement (Variables|Default|GetOwnerCharacter))))

(fn SpawnShockBeam
  (Class|AuroraBeamSpell|TraceFirstTarget (Variables|Default|GetMouseHitLocation))
  (bind _returnvalue (Class|CombatInterface|GetWeapon(Message) (Variables|Default|GetOwnerCharacter)))
  (Variables|Default|SetFirstTargetCueParams (Ability|GameplayCue|MakeGameplayCueParameters :Location (Variables|Default|GetMouseHitLocation) :SourceObject (Variables|Default|GetMouseHitActor) :TargetAttachComponent _returnvalue))
  ;[1 0.6399 0.3618] Combat Interface Valid Check
  (bind _output_get (Variables|Default|SetFirstTargetImplementsCombatInerface (Utilities|DoesObjectImplementInterface (Variables|Default|GetMouseHitActor) "/Script/Aurora.CombatInterface")))
  (if _output_get
    (LocalVariables|SetCueTarget (Variables|Default|GetMouseHitActor))
    (else
      (LocalVariables|SetCueTarget (Ability|GetAvatarActorfromActorInfo))))
  (GameplayCue|AddGameplayCueOnActor(Looping) (LocalVariables|GetCueTarget) "(TagName=\"GameplayCue.ShockLoop\")" (Variables|Default|GetFirstTargetCueParams))
  (if (Variables|Default|GetFirstTargetImplementsCombatInerface)
    (bind _outadditionaltargets (Class|AuroraBeamSpell|StoreAdditionalTargets))
    (bind _output_get_2 (Variables|Default|SetAdditionalTargets _outadditionaltargets))
    (for _array_element _output_get_2
      (CallFunction|AddShockLoopCuetoAddTarget _array_element))))

(fn AddShockLoopCuetoAddTarget
  (params (AdditionalTarget :type Actor%20Object%20Reference))
  (LocalVariables|SetTargetActor AdditionalTarget)
  (Utilities|Map|Add (Variables|Default|GetAdditionalActorsToCueParams) (LocalVariables|GetTargetActor) (Ability|GameplayCue|MakeGameplayCueParameters :Location (Transformation|GetActorLocation (LocalVariables|GetTargetActor)) :SourceObject (LocalVariables|GetTargetActor) :TargetAttachComponent (Variables|/Script/Engine.Actor|GetRootComponent (Variables|Default|GetMouseHitActor))))
  (GameplayCue|AddGameplayCueOnActor(Looping) (LocalVariables|GetTargetActor) "(TagName=\"GameplayCue.ShockLoop\")" (Ability|GameplayCue|MakeGameplayCueParameters :Location (Transformation|GetActorLocation (LocalVariables|GetTargetActor)) :SourceObject (LocalVariables|GetTargetActor) :TargetAttachComponent (Variables|/Script/Engine.Actor|GetRootComponent (Variables|Default|GetMouseHitActor)))))

(fn RemoveLoopCurefromAddTarget
  (params (Additional%20Target :type Actor%20Object%20Reference))
  (LocalVariables|SetTarget Additional%20Target)
  (if (.ReturnValue (Utilities|Map|Find (Variables|Default|GetAdditionalActorsToCueParams) (LocalVariables|GetTarget)))
    (GameplayCue|RemoveGameplayCueOnActor(Looping) (LocalVariables|GetTarget) "(TagName=\"GameplayCue.ShockLoop\")" (.Value (Utilities|Map|Find (Variables|Default|GetAdditionalActorsToCueParams) (LocalVariables|GetTarget))))))

(fn ApplyDamage
  (Utilities|FlowControl|Sequence
    (:then_0
      (CallFunction|ApplyDamageSingleTarget (Variables|Default|GetMouseHitActor)))
    (:then_1
      (for _array_element (Variables|Default|GetAdditionalTargets)
        (CallFunction|ApplyDamageSingleTarget _array_element)))))

(fn ApplyDamageSingleTarget
  (params (Actor :type Actor%20Object%20Reference))
  (bind _output_get (LocalVariables|SetDamagedTarget Actor))
  (Utilities|IsValid _output_get
    (:Is%20Valid
      (Utilities|FlowControl|Sequence
        (:then_0
          (bind _output_get_2 (LocalVariables|SetASC (Ability|GetAbilitySystemComponentfromActorInfo)))
          (Utilities|IsValid _output_get_2
            (:Is%20Valid
              (bind _returnvalue (Ability|GameplayEffect|AssignTagSetbyCallerMagnitude (GameplayEffects|MakeOutgoingSpec (LocalVariables|GetASC) (Variables|Default|GetDamageEffectClass) (Math|Conversions|ToFloat(Integer) (Ability|GetAbilityLevel)) (GameplayEffects|MakeEffectContext (LocalVariables|GetASC))) "(TagName=\"Damage.Lightning\")" (Class|AuroraDamageGameplayAbility|GetDamageatLevel)))
              (LocalVariables|SetEffectSpec _returnvalue))))
        (:then_1
          (Utilities|IsValid (Ability|GetAbilitySystemComponent (LocalVariables|GetDamagedTarget))
            (:Is%20Valid
              (Class|AuroraAbilitySystemLibrary|ApplyDamageEffect (Class|AuroraDamageGameplayAbility|MakeDamageEffectParamsfromClassDefaults (LocalVariables|GetDamagedTarget) "0, 0, 0")))))))))

(fn ClearTimeandEndAbility
  (Utilities|FlowControl|Sequence
    (:then_0
      (Utilities|Time|ClearandInvalidateTimerbyHandle (Variables|Default|GetDamageAndCostTimer)))
    (:then_1
      (CallFunction|PreparetoEndAbility))
    (:then_2
      (Ability|CommitAbilityCooldown false))
    (:then_3
      (Utilities|Array|Clear (Variables|Default|GetAdditionalTargets))
      (Utilities|Map|Clear (Variables|Default|GetAdditionalActorsToCueParams))
      (Variables|Default|SetTime%20Held 0.0)
      (Variables|Default|SetMouseHitActor 0))
    (:then_4
      (Variables|Default|SetFirstTargetImplementsCombatInerface false)
      (Ability|EndAbility))))