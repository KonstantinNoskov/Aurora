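; Enemy melee attack ability that turns toward the combat target and plays a random tagged attack montage.
; On the montage's gameplay event, it searches for living players within the melee radius around the montage's combat socket and damages non-friendly ones.
; A hit triggers the MeleeImpact gameplay cue at that socket, tagged with the montage tag.
; The instanced-per-actor ability resets its hit flag on each activation.
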(event Ability|EventActivateAbility
  (Utilities|FlowControl|Sequence
    (:then_0
      ;[1 0.9824 0] Reset variables from the last usage since instance policy set to instanced per actor.
      (Variables|Default|SetHasHitTarget false))
    (:then_1
      (Variables|Default|SetSourceActor (Ability|GetAvatarActorfromActorInfo)))
    (:then_2
      (CallFunction|GetAttackTargetLocation)
      (bind _ascombat_interface (Utilities|Casting|CastToCombatInterface (Variables|Default|GetSourceActor)))
      (bind _output_get (Variables|Default|SetSourceCombatInterface _ascombat_interface))
      (Class|CombatInterface|UpdateFacingTarget _output_get (Variables|Default|GetAttackTargetLocation))
      (bind _returnvalue (Class|CombatInterface|GetAttackMontages(Message) (Variables|Default|GetSourceActor)))
      (bind _output_get_2 (Variables|Default|SetTaggedMontage (Class|AuroraDamageGameplayAbility|GetRandomTaggedMontagefromArray _returnvalue)))
      (|PlayMontageandWaitProxy "None" (.Montage (Utilities|Struct|BreakTaggedMontage _output_get_2)) 1.0 "None" true 1.0 0.0 false
        (:then
          (Ability|Tasks|WaitGameplayEvent (.MontageTag (Utilities|Struct|BreakTaggedMontage _output_get_2)) 0
            (:EventReceived
              (bind _returnvalue_2 (Class|CombatInterface|GetCombatSocketLocation (Variables|Default|GetSourceCombatInterface) (.SocketTag (Utilities|Struct|BreakTaggedMontage _output_get_2))))
              (bind _output_get_3 (Variables|Default|SetWeaponTipSocketLocation _returnvalue_2))
              (bind _outoverlappingactors (Class|AuroraAbilitySystemLibrary|GetAlivePlayersWithinRadius (Variables|Default|GetSourceActor) (Utilities|Array|MakeArray (Variables|Default|GetSourceActor)) (Class|CombatInterface|GetMeleeAttackRadius (Variables|Default|GetSourceCombatInterface)) (Variables|Default|GetWeaponTipSocketLocation)))
              (if (Utilities|Array|IsNotEmpty _outoverlappingactors)
                (for _array_element _outoverlappingactors
                  (if (not (Class|AuroraAbilitySystemLibrary|IsActorsFriendly _array_element (Variables|Default|GetSourceActor)))
                    (Class|AuroraDamageGameplayAbility|CauseDamage _array_element)
                    (Variables|Default|SetHasHitTarget true)
                    (Ability|EndAbility)))
                (if (Variables|Default|GetHasHitTarget)
                  (bind _returnvalue_3 (Class|TargetInterface|GetCombatTarget(Message) (Variables|Default|GetSourceActor)))
                  (Class|GameplayAbility|ExecuteGameplayCuewithParams "(TagName=\"GameplayCue.MeleeImpact\")" (Ability|GameplayCue|MakeGameplayCueParameters :AggregatedSourceTags (GameplayTags|MakeGameplayTagContainerfromTag (.MontageTag (Utilities|Struct|BreakTaggedMontage (Variables|Default|GetTaggedMontage)))) :Location (Variables|Default|GetWeaponTipSocketLocation) :EffectCauser (Variables|Default|GetSourceActor) :SourceObject _returnvalue_3)))
                (Ability|EndAbility)
                (else
                  (Ability|EndAbility))))))
        (:OnCompleted
          (Ability|EndAbility :!label _label))
        (:OnInterrupted
          (goto _label))
        (:OnCancelled
          (goto _label))))))

(fn GetAttackTargetLocation
  (bind _returnvalue (Class|TargetInterface|GetCombatTarget(Message) (Variables|Default|GetSourceActor)))
  (Variables|Default|SetAttackTargetLocation (Transformation|GetActorLocation _returnvalue)))