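; Gameplay ability for enemy ranged attacks that fires a projectile at the avatar's current combat target.
; On activation it captures the target's location, updates facing toward it and plays a random tagged montage from the avatar.
; The montage's gameplay event triggers the projectile spawn from the tagged socket with pitch override.
; The ability ends shortly after firing or when the montage finishes or is interrupted, without stopping the montage.
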(event Ability|EventActivateAbility
  (Variables|Default|SetSourceActor (Ability|GetAvatarActorfromActorInfo))
  (CallFunction|GetAttackTargetLocation)
  (Class|CombatInterface|UpdateFacingTarget(Message) (Variables|Default|GetSourceActor) (Variables|Default|GetAttackTargetLocation))
  (bind _returnvalue (Class|CombatInterface|GetAttackMontages(Message) (Variables|Default|GetSourceActor)))
  (bind _output_get (Variables|Default|SetTaggedMontage (Class|AuroraDamageGameplayAbility|GetRandomTaggedMontagefromArray _returnvalue)))
  (|PlayMontageandWaitProxy "None" (.Montage (Utilities|Struct|BreakTaggedMontage _output_get)) 1.0 "None" false 1.0 0.0 false
    (:then
      (Ability|Tasks|WaitGameplayEvent (.MontageTag (Utilities|Struct|BreakTaggedMontage _output_get)) 0
        (:EventReceived
          (Class|AuroraProjectileSpell|SpawnProjectile (Variables|Default|GetAttackTargetLocation) (.SocketTag (Utilities|Struct|BreakTaggedMontage _output_get)) true 0.0)
          (Utilities|FlowControl|Delay 0.05)
          (Ability|EndAbility))))
    (:OnCompleted
      (Ability|EndAbility :!label _label))
    (:OnInterrupted
      (goto _label))
    (:OnCancelled
      (goto _label))))

(fn GetAttackTargetLocation
  (bind _returnvalue (Class|TargetInterface|GetCombatTarget(Message) (Variables|Default|GetSourceActor)))
  (Variables|Default|SetAttackTargetLocation (Transformation|GetActorLocation _returnvalue)))