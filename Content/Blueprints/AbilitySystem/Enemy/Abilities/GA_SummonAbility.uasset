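; GA_SummonAbility is an enemy gameplay ability in which a shaman summons random minions.
; It turns the avatar toward the player, plays the summon montage and waits for its gameplay event to get and shuffle spawn locations.
; A Delay-paced loop plays a ground effect at each location, then spawns a minion with its default controller.
; The avatar's minion count rises on each spawn and falls through a bound OnDestroyed event.
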(event Custom|OnDestroyed_Event
  (params (DestroyedActor :type Actor%20Object%20Reference))
  (Class|CombatInterface|IncrementMinionCount(Message) (Ability|GetAvatarActorfromActorInfo) -1))

(event Ability|EventActivateAbility
  (bind _returnvalue (Class|AuroraSummonAbility|GetRandomMinionClass))
  (CallFunction|FacingPlayer)
  (|PlayMontageandWaitProxy "None" "/Game/Assets/Enemies/Shaman/Animations/AM_Shaman_Summon.AM_Shaman_Summon" 1.0 "None" true 1.0 0.0 false
    (:then
      (Ability|Tasks|WaitGameplayEvent "(TagName=\"Montage.Attack.2\")" 0
        (:EventReceived
          (bind _returnvalue_2 (Class|AuroraSummonAbility|GetSpawnLocations))
          (Variables|Default|SetSpawnLocations _returnvalue_2)
          (Utilities|Array|Shuffle (Variables|Default|GetSpawnLocations))
          (if (< (Variables|Default|GetSpawnLocationIndex) (Utilities|Array|Length (Variables|Default|GetSpawnLocations))) :!label _label
            (Niagara|SpawnSystematLocation "/Game/Assets/Effects/Combat/NS_GroundSummon.NS_GroundSummon" (Utilities|Array|Get(acopy) (Variables|Default|GetSpawnLocations) (Variables|Default|GetSpawnLocationIndex)))
            (Utilities|FlowControl|Delay 0.2)
            (Variables|Default|SetCurrentSpawnLocation (+ (Utilities|Array|Get(acopy) (Variables|Default|GetSpawnLocations) (Variables|Default|GetSpawnLocationIndex)) (Math|Vector|MakeVector 0.0 0.0 (Components|Capsule|GetScaledCapsuleHalfHeight (Variables|/Script/Engine.Character|GetCapsuleComponent _returnvalue)))))
            (bind _returnvalue_3 (Game|SpawnActorfromClass (Utilities|GetClass _returnvalue) (Math|Transform|MakeTransform (Variables|Default|GetCurrentSpawnLocation) (Math|Rotator|FindLookatRotation (Transformation|GetActorLocation (Ability|GetAvatarActorfromActorInfo)) (+ (Utilities|Array|Get(acopy) (Variables|Default|GetSpawnLocations) (Variables|Default|GetSpawnLocationIndex)) (Math|Vector|MakeVector 0.0 0.0 (Components|Capsule|GetScaledCapsuleHalfHeight (Variables|/Script/Engine.Character|GetCapsuleComponent _returnvalue))))) "1.000000,1.000000,1.000000") "AlwaysSpawn" "MultiplyWithRoot" 0 0))
            (Game|AssignOnDestroyed _returnvalue_3 (delegate Custom|OnDestroyed_Event))
            (Pawn|SpawnDefaultController _returnvalue_3)
            (Class|CombatInterface|IncrementMinionCount(Message) (Ability|GetAvatarActorfromActorInfo) 1)
            (Math|Integer|IncrementInt (Variables|Default|GetSpawnLocationIndex)
              (:%20%20
                (Utilities|FlowControl|Delay 0.2)
                (goto _label)))))))))

(fn FacingPlayer
  (bind _outactors (Actor|GetAllActorswithTag "Player"))
  (bind _output_get (Variables|Default|SetTargetActor (Utilities|Array|Get(acopy) _outactors)))
  (Class|CombatInterface|UpdateFacingTarget(Message) (Ability|GetAvatarActorfromActorInfo) (Transformation|GetActorLocation _output_get)))