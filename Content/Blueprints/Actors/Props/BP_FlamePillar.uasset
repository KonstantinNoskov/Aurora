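; BP_FlamePillar is a flame pillar prop whose fire light varies in intensity over time.
; On BeginPlay it randomly picks one of two intensity timelines, then picks again each time one finishes, so the variation continues without a fixed sequence.
; Each timeline update passes its curve value to ScaleFlameIntensity, which multiplies it by a base intensity and applies it to the FireLight.
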(event Custom|StartTimeLine_2
  (bind _flameintensity (Timeline|FlameIntensity_2 PlayFromStart)
    (:Update
      (CallFunction|ScaleFlameIntensity _flameintensity))
    (:Finished
      (CallFunction|ChooseTimeLine))))

(event Custom|StartTimeLine_1
  (bind _flameintensity (Timeline|FlameIntensity_1 PlayFromStart)
    (:Update
      (CallFunction|ScaleFlameIntensity _flameintensity))
    (:Finished
      (CallFunction|ChooseTimeLine))))

(event Custom|ChooseTimeLine
  (switch int (Math|Random|RandomIntegerinRange 0 1)
    (:0
      (CallFunction|StartTimeLine1))
    (:1
      (CallFunction|StartTimeLine2))))

(event EventBeginPlay
  (CallFunction|ChooseTimeLine))

(fn ConstructionScript)

(fn ScaleFlameIntensity
  (params (Intensity :type Float%20%28double-precision%29))
  (Rendering|Components|Light|SetIntensity (Variables|Default|GetFireLight) (* Intensity (Variables|Default|GetBaseFireLightIntensity))))