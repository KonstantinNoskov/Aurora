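; BP_Test_Cube is a test actor that visualizes its local axes with debug arrows and on-screen prints.
; Each Tick, SetAxisY draws the forward arrow in green and SetAxisX draws the right arrow in red.
; A blue third arrow uses the cross product of ForwardVector and RightVector.
; ForwardVector is never assigned here, and RightVector stores the arrow's world endpoint rather than a direction, so that cross product is not the up axis.
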(event EventTick
  (params (DeltaSeconds :type Float%20%28single-precision%29))
  (bind _returnvalue (Transformation|GetActorLocation))
  (bind _arrowdistance (Variables|Default|GetArrowDistance))
  (CallFunction|SetAxisY)
  (CallFunction|SetAxisX)
  (Development|PrintString (Utilities|String|ToString(Vector) (Variables|Default|GetForwardVector)) true true "(R=1.000000,G=0.000000,B=0.000000,A=1.000000)" 0.0 "2")
  (Rendering|Debug|DrawDebugArrow _returnvalue (+ _returnvalue (* (Math|Vector|CrossProduct (Variables|Default|GetForwardVector) (Variables|Default|GetRightVector)) (Math|Vector|MakeVector _arrowdistance _arrowdistance _arrowdistance))) (Variables|Default|GetArrowSize) "(R=0.000000,G=0.210234,B=1.000000,A=1.000000)" 0.0 (Variables|Default|GetArrowThickness)))

(fn ConstructionScript)

(fn SetAxisY
  (bind _returnvalue (Transformation|GetActorForwardVector))
  (bind _returnvalue_2 (Transformation|GetActorLocation))
  (bind _arrowdistance (Variables|Default|GetArrowDistance))
  (bind _returnvalue_3 (* _returnvalue (Math|Vector|MakeVector _arrowdistance _arrowdistance _arrowdistance)))
  (bind _returnvalue_4 (+ _returnvalue_2 _returnvalue_3))
  (Development|PrintString (Utilities|String|ToString(Vector) (Math|Vector|Normalize _returnvalue_4)) true true "(R=0.000000,G=1.000000,B=0.000000,A=1.000000)" 0.0 "1")
  (Rendering|Debug|DrawDebugArrow _returnvalue_2 _returnvalue_4 (Variables|Default|GetArrowSize) "(R=0.000000,G=1.000000,B=0.133649,A=1.000000)" 0.0 (Variables|Default|GetArrowThickness))
  (return))

(fn SetAxisX
  (bind _returnvalue (Transformation|GetActorLocation))
  (bind _arrowdistance (Variables|Default|GetArrowDistance))
  (bind _output_get (Variables|Default|SetRightVector (+ _returnvalue (* (Transformation|GetActorRightVector) (Math|Vector|MakeVector _arrowdistance _arrowdistance _arrowdistance)))))
  (Rendering|Debug|DrawDebugArrow _returnvalue _output_get (Variables|Default|GetArrowSize) "(R=1.000000,G=0.000000,B=0.000000,A=1.000000)" 0.0 (Variables|Default|GetArrowThickness)))