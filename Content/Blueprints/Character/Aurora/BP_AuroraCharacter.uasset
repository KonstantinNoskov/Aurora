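; BP_AuroraCharacter is the Aurora character Blueprint, handling highlighting, attack facing and fading of objects that overlap its Box component.
; Highlight events toggle custom depth on the mesh, and UpdateFacingTarget feeds a location to the FacingTarget motion warp target for attacks.
; SetinShockLoop stores the shock loop state.
; Box overlaps send fade-out and fade-in messages to actors implementing BPI_FadeInterface.
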(event OnComponentBeginOverlap(Box)
  (params (OverlappedComponent :type Primitive%20Component%20Object%20Reference) (OtherActor :type Actor%20Object%20Reference) (OtherComp :type Primitive%20Component%20Object%20Reference) (OtherBodyIndex :type Integer) (bFromSweep :type Boolean) (SweepResult :type Hit%20Result%20Structure%20%28by%20ref%29))
  ;[0.3146 0.5071 1] Call fade object to fade out if possible
  (if (Utilities|DoesObjectImplementInterface OtherActor "/Game/Blueprints/Actors/FadeProccess/BPI_FadeInterface.BPI_FadeInterface_C")
    (Class|BPIFadeInterface|FadeOut(Message) OtherActor)))

(event OnComponentEndOverlap(Box)
  (params (OverlappedComponent :type Primitive%20Component%20Object%20Reference) (OtherActor :type Actor%20Object%20Reference) (OtherComp :type Primitive%20Component%20Object%20Reference) (OtherBodyIndex :type Integer))
  ;[0.3146 0.5071 1] Call fade object to fade out if possible
  (if (Utilities|DoesObjectImplementInterface OtherActor "/Game/Blueprints/Actors/FadeProccess/BPI_FadeInterface.BPI_FadeInterface_C")
    (Class|BPIFadeInterface|Fadein(Message) OtherActor)))

(event EventSetinShockLoop
  (params (bInLoop :type Boolean))
  (Variables|Default|SetInShockLoop bInLoop))

(event EventBeginPlay)

(event EventHighLightActor
  (Rendering|SetRenderCustomDepth (Variables|Character|GetMesh) true))

(event EventUpdateFacingTarget
  (params (Target :type Vector%20%28by%20ref%29 :default "0, 0, 0"))
  ;[1 0.2116 0.4129] Facing to a target when attack
  (Class|MotionWarpingComponent|AddorUpdateWarpTargetfromLocation (Variables|Components|GetMotionWarping) "FacingTarget" Target))

(event EventUnHighLightActor
  (Rendering|SetRenderCustomDepth (Variables|Character|GetMesh) false))

(fn ConstructionScript)