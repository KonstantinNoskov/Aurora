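; BP_AuroraMainMenu is the main menu scene actor that opens the menu and animates its backdrop.
; On BeginPlay it plays menu music, adds the WBP_MainMenu widget, switches to UI-only input and shows the cursor.
; Each tick it bobs the FireBall vertically around its starting location with a sine of speed-scaled elapsed time, and slowly spins the magic circle decal.
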(event EventBeginPlay
  (bind _returnvalue (Game|GetPlayerController 0))
  (Variables|Default|SetFireBallInitialLocation (Transformation|GetWorldLocation (Variables|Default|GetFireBall)))
  (Audio|PlaySound2D "/Game/Assets/Sounds/Music/Music_MainMenu.Music_MainMenu" 1.0 1.0 0.0 0 0)
  (bind _returnvalue_2 (UserInterface|CreateWidget "/Game/UI/MainMenu/WBP_MainMenu.WBP_MainMenu_C"))
  (UserInterface|Viewport|AddtoViewport _returnvalue_2 0)
  (Input|SetInputModeUIOnly _returnvalue _returnvalue_2 "DoNotLock" false)
  (Variables|/Script/Engine.PlayerController|SetbShowMouseCursor _returnvalue true))

(event Collision|EventActorBeginOverlap
  (params (OtherActor :type Actor%20Object%20Reference)))

(event EventTick
  (params (DeltaSeconds :type Float%20%28single-precision%29))
  (Utilities|FlowControl|Sequence
    (:then_0
      (CallFunction|UpdateTime (Utilities|Time|GetWorldDeltaSeconds))
      (Transformation|SetWorldLocation (Variables|Default|GetFireBall) (+ (Variables|Default|GetFireBallInitialLocation) (Math|Vector|MakeVector 0.0 0.0 (CallFunction|SinTime))) false false))
    (:then_1
      (Transformation|AddLocalRotation (Variables|Default|GetMagicCIrcleDecal) (Math|Rotator|MakeRotator (* (Utilities|Time|GetWorldDeltaSeconds) 1.5) 0.0 0.0) false false))))

(fn ConstructionScript)

(fn UpdateTime
  (params (DeltaSeconds :type Float%20%28double-precision%29))
  (Utilities|FlowControl|Sequence
    (:then_0
      (Variables|Default|SetElapsedTime (+ (* DeltaSeconds (Variables|Default|GetFireSpeed)) (Variables|Default|GetElapsedTime))))
    (:then_1)
    (:then_2
      (return (Variables|Default|GetElapsedTime)))))

(fn SinTime
  (Utilities|FlowControl|Sequence
    (:then_0
      (LocalVariables|SetSinAmplitude (* (Math|Trig|Sin(Radians) (Variables|Default|GetElapsedTime)) (Variables|Default|GetFireAmplitude))))
    (:then_1)
    (:then_2
      (return (LocalVariables|GetSinAmplitude)))))