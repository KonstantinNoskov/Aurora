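; BP_Enemy is an enemy character Blueprint that handles loot drops, death dissolve visuals and motion-warped facing.
; SpawnLoot rolls items from loot tiers, then a looping timer spawns them one by one, evenly fanned around the enemy at random distances.
; Spawned AuroraEffectActors take the enemy's level when the item's override flag is set.
; Timelines drive a Dissolve material parameter on body and weapon, and UpdateFacingTarget feeds a motion warp target.
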(event Custom|SpawnLootItem
  (bind _lootitems (Variables|Default|GetLootItems))
  (bind _spawnlootcount (Variables|Default|GetSpawnLootCount))
  (bind _output (Utilities|Array|Get(acopy) _lootitems _spawnlootcount))
  (bind (_lootclass _blootleveloverride) (Utilities|Struct|BreakLootItem _output))
  ;[1 0.9055 0.2271] Spawn Loot
  (if (< (Variables|Default|GetSpawnLootCount) (Utilities|Array|Length (Variables|Default|GetLootItems)))
    (Variables|Default|SetbLevelOverride _blootleveloverride)
    (bind _returnvalue (Game|SpawnActorfromClass _lootclass (CallFunction|GetLootTransform (Variables|Default|GetSpawnLootCount)) "AlwaysSpawn" "MultiplyWithRoot" 0 0))
    (Utilities|FlowControl|Sequence
      (:then_0
        (Math|Integer|IncrementInt (Variables|Default|GetSpawnLootCount)))
      (:then_1
        (CallFunction|SetLootLevel _returnvalue)))
    (else
      (Utilities|Time|ClearandInvalidateTimerbyHandle (Variables|Default|GetLootTimer)))))

(event EventStartWeaponDissolveTimeLine
  (params (DynamicMaterialInstance :type Material%20Instance%20Dynamic%20Object%20Reference))
  (bind _dissolvetrack (Timeline|Weapon%20Dissolve%20Timeline Play)
    (:Update
      (Rendering|Material|SetScalarParameterValue DynamicMaterialInstance "Dissolve" _dissolvetrack :!class /Script/Engine.MaterialInstanceDynamic))))

(event EventUpdateFacingTarget
  (params (Target :type Vector%20%28by%20ref%29 :default "0, 0, 0"))
  (Class|MotionWarpingComponent|AddorUpdateWarpTargetfromLocation (Variables|Default|GetMotionWarping) "FacingTarget" Target))

(event EventSpawnLoot
  ;[1 0.9055 0.2271] Spawn Loot
  (bind _returnvalue (Class|AuroraAbilitySystemLibrary|GetLootTiers self))
  (Utilities|IsValid _returnvalue
    (:Is%20Valid
      (bind _returnvalue_2 (Class|LootTiers|GetLootItems _returnvalue))
      (bind _output_get (Variables|Default|SetLootItems _returnvalue_2))
      (Variables|Default|SetLootRotations (CallFunction|GetLootRotations _output_get))
      (Variables|Default|SetSpawnLootCount 0)
      (bind _returnvalue_3 (Utilities|Time|SetTimerbyEvent (delegate Custom|SpawnLootItem) 0.1 true))
      (Variables|Default|SetLootTimer _returnvalue_3)
      (CallFunction|SpawnLootItem))))

(event EventStartDissolveTimeLine
  (params (DynamicMaterialInstance :type Material%20Instance%20Dynamic%20Object%20Reference))
  (bind _dissolvetrack (Timeline|Dissolve%20Time%20Line Play)
    (:Update
      (Rendering|Material|SetScalarParameterValue DynamicMaterialInstance "Dissolve" _dissolvetrack :!class /Script/Engine.MaterialInstanceDynamic))))

(fn ConstructionScript)

(fn GetLootRotations
  (params (TargetArray :type Array%20of%20Loot%20Item%20Structures))
  (bind _returnvalue (Class|AuroraAbilitySystemLibrary|EvenlySpacedRotators (Transformation|GetActorForwardVector) (Math|Vector|VectorUp) 3.6e+02 (Utilities|Array|Length TargetArray)))
  (return _returnvalue))

(fn GetLootTransform
  (params (Loot%20Count :type Integer))
  (return (Math|Transform|MakeTransform (+ (* (Math|Vector|GetForwardVector (Utilities|Array|Get(acopy) (Variables|Default|GetLootRotations) Loot%20Count)) (Math|Random|RandomFloatinRange (Variables|Default|GetMinSpawnDistance) (Variables|Default|GetMaxSpawnDistance))) (Transformation|GetActorLocation)) (Utilities|Array|Get(acopy) (Variables|Default|GetLootRotations) (Variables|Default|GetSpawnLootCount)))))

(fn SetLootLevel
  (params (Spawned%20Loot :type Object%20Object%20Reference))
  (bind _asaurora_effect_actor (Utilities|Casting|CastToAuroraEffectActor Spawned%20Loot))
  (Utilities|IsValid _asaurora_effect_actor
    (:Is%20Valid
      (if (Variables|Default|GetbLevelOverride)
        (Variables|/Script/Aurora.AuroraEffectActor|SetActorLevel _asaurora_effect_actor (Math|Conversions|ToFloat(Integer) (Variables|Default|GetLevel)))))))